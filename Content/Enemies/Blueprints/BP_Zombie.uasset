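; Zombie enemy Blueprint that flees from wheeled vehicles it sees or hears through PawnSensing.
; RunAway ignores anything that is not a WheeledVehicle, then projects a point directly away from the vehicle at the zombie's own height.
; AI MoveTo heads for a random reachable point around that spot and calls RunAway again on success or failure, so the flight repeats indefinitely.
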(event OnSeePawn(PawnSensing)
  (params (Pawn :type Pawn%20Object%20Reference))
  (CallFunction|RunAway Pawn))

(event OnHearNoise(PawnSensing)
  (params (Instigator :type Pawn%20Object%20Reference) (Location :type Vector%20%28by%20ref%29 :default "0, 0, 0") (Volume :type Float%20%28single-precision%29))
  (CallFunction|RunAway Instigator))

(event Custom|RunAway
  (params (VehicleRef :type Object%20Object%20Reference))
  (bind _returnvalue (Transformation|GetActorLocation))
  (bind _aswheeled_vehicle (Utilities|Casting|CastToWheeledVehicle VehicleRef))
  (AI|AIMoveTo self (.RandomLocation (AI|Navigation|GetRandomReachablePointinRadius (Math|Vector|MakeVector (.X (Math|Vector|BreakVector (+ _returnvalue (* (Math|Vector|GetForwardVector (Math|Rotator|FindLookatRotation _returnvalue (Transformation|GetActorLocation _aswheeled_vehicle))) -5e+02)))) (.Y (Math|Vector|BreakVector (+ _returnvalue (* (Math|Vector|GetForwardVector (Math|Rotator|FindLookatRotation _returnvalue (Transformation|GetActorLocation _aswheeled_vehicle))) -5e+02)))) (.Z (Math|Vector|BreakVector _returnvalue))) 5e+02 0 0)) 0 5.0 false
    (:OnSuccess
      _)
    (:OnFail
      _))
  (CallFunction|RunAway _aswheeled_vehicle))

(fn ConstructionScript)