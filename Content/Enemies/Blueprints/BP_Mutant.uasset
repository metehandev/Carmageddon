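; Mutant enemy Blueprint that senses pawns by sight or sound and turns to face where it is moving.
; PawnSensing events feed Chase, which only casts the pawn to WheeledVehicle and takes no further action.
; While moving, Tick smoothly interpolates yaw toward the desired velocity.
; MoveToVehicle sends the AI to a random navigable point near a vehicle, but nothing in this file calls it.
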(event OnSeePawn(PawnSensing)
  (params (Pawn :type Pawn%20Object%20Reference))
  (CallFunction|Chase Pawn))

(event OnHearNoise(PawnSensing)
  (params (Instigator :type Pawn%20Object%20Reference) (Location :type Vector%20%28by%20ref%29 :default "0, 0, 0") (Volume :type Float%20%28single-precision%29))
  (CallFunction|Chase Instigator))

(event Custom|Chase
  (params (Pawn :type Pawn%20Object%20Reference))
  (bind _aswheeled_vehicle (Utilities|Casting|CastToWheeledVehicle Pawn)))

(event EventTick
  (params (DeltaSeconds :type Float%20%28single-precision%29))
  (if (> (Math|Vector|VectorLength (Transformation|GetVelocity)) 1e+01)
    (bind _desired_velocity (CallFunction|GetDesiredVelocity))
    (Transformation|SetActorRotation (Math|Rotator|MakeRotator 0.0 0.0 (.yaw (Math|Interpolation|RInterpTo (Transformation|GetActorRotation) (Math|Conversions|RotationFromXVector _desired_velocity) DeltaSeconds 1.0))))))

(fn ConstructionScript)

(fn MovetoVehicle
  (params (Pawn :type Object%20Object%20Reference))
  (bind _aswheeled_vehicle (Utilities|Casting|CastToWheeledVehicle Pawn))
  (bind _randomlocation (Class|NavigationSystemV1|GetRandomLocationinNavigableRadius (Pawn|GetNavAgentLocation _aswheeled_vehicle) 1.5e+02 0 0))
  (AI|Navigation|SimpleMovetoLocation (AI|GetAIController self) _randomlocation)
  (return))